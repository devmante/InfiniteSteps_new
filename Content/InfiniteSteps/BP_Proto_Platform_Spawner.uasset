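; Spawner for an infinite stair-stepping game that builds a zigzag chain of platforms and resolves the player's direction input against it.
; BeginPlay seeds the chain, with each step randomly offset to either side by mirroring the Y offset.
; A correct input shifts the stack down, culls old platforms, teleports the player, reduces that platform's durability and spawns another.
; A wrong input ends the game through InfiniteStepsGameMode.
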(event EventBeginPlay
  (Variables|Default|SetLastPlatformLoc (Transformation|GetActorLocation))
  (for _index (range 0 9)
    (CallFunction|SpawnPlatform))
  (Variables|Default|SetNextPlatform (Utilities|Array|Get(acopy) (Variables|Default|GetPlatforms))))

(fn ConstructionScript)

(fn SpawnPlatform
  (bind _platformoffset (Variables|Default|GetPlatformOffset))
  (if (Math|Random|RandomBoolwithWeight 0.5)
    (bind _returnvalue (Game|SpawnActorfromClass "/Game/InfiniteSteps/BP_Proto_Platform.BP_Proto_Platform_C" (Math|Conversions|ToTransform(Vector) (+ (Variables|Default|GetLastPlatformLoc) (Variables|Default|GetPlatformOffset))) "Undefined" 0 "NewEnumerator0" 0))
    (Variables|Default|SetLastPlatformLoc (+ (Variables|Default|GetLastPlatformLoc) (Variables|Default|GetPlatformOffset)))
    (Utilities|Array|Add (Variables|Default|GetPlatforms) _returnvalue)
    (else
      (bind _returnvalue_2 (Game|SpawnActorfromClass "/Game/InfiniteSteps/BP_Proto_Platform.BP_Proto_Platform_C" (Math|Conversions|ToTransform(Vector) (+ (Variables|Default|GetLastPlatformLoc) (Math|Vector|MakeVector (.x _platformoffset) (* (.y _platformoffset) -1.0) (.z _platformoffset)))) "Undefined" 0 "NewEnumerator1" 0))
      (Variables|Default|SetLastPlatformLoc (+ (Variables|Default|GetLastPlatformLoc) (Math|Vector|MakeVector (.x _platformoffset) (* (.y _platformoffset) -1.0) (.z _platformoffset))))
      (Utilities|Array|Add (Variables|Default|GetPlatforms) _returnvalue_2))))

(fn HandlePlayerInput
  (params (Direction :type Enum_Platform_Direction%20Enum :default "NewEnumerator0"))
  (if (Utilities|Enum|Equal(Enum) Direction (Variables|/Game/InfiniteSteps/BP_Proto_Platform.BP_Proto_Platform_C|GetDirection (Variables|Default|GetNextPlatform)))
    (CallFunction|ShiftPlatforms)
    (Transformation|SetActorLocation (Variables|Default|GetPlayerRef) (Transformation|GetActorLocation (Variables|Default|GetNextPlatform)) false true)
    (Default|DecreaseDurability (Variables|Default|GetNextPlatform))
    (bind _output_get (Variables|Default|SetCurrentIndex (Utilities|Array|FindItem (Variables|Default|GetPlatforms) (Variables|Default|GetNextPlatform))))
    (Variables|Default|SetNextPlatform (Utilities|Array|Get(acopy) (Variables|Default|GetPlatforms) (+ _output_get 1)))
    (CallFunction|SpawnPlatform)
    (else
      (bind _asinfinite_steps_game_mode (Utilities|Casting|CastToInfiniteStepsGameMode (Game|GetGameMode)))
      (Default|EndGame _asinfinite_steps_game_mode))))

(fn ShiftPlatforms
  (bind _platforms (Variables|Default|GetPlatforms))
  (CallFunction|DeleteOldestPlatform)
  (for _array_element (Variables|Default|GetPlatforms)
    (Transformation|AddActorWorldOffset _array_element "0, 0,-20.000000" false true))
  (Variables|Default|SetLastPlatformLoc (Transformation|GetActorLocation (Utilities|Array|Get(acopy) _platforms (Utilities|Array|LastIndex _platforms)))))

(fn DeleteOldestPlatform
  (bind _platforms (Variables|Default|GetPlatforms))
  (if (>= (Utilities|Array|Length (Variables|Default|GetPlatforms)) 15)
    (Actor|DestroyActor (Utilities|Array|Get(acopy) _platforms))
    (Utilities|Array|RemoveIndex _platforms)))