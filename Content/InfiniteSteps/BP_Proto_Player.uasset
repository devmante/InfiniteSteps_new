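; BP_Proto_Player is a prototype player for InfiniteSteps that turns Left and Right input presses into stepping directions for a platform spawner.
; Each press calls Rotate, then forwards its direction to PlatformSpawnerRef through HandlePlayerInput.
; Rotate snaps BasicCharacter to one of two fixed yaw angles by direction.
; Both input events pass Left to Rotate, so the right-facing branch is never reached from this graph.
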(event EventBeginPlay)

(event Collision|EventActorBeginOverlap
  (params (OtherActor :type Actor%20Object%20Reference)))

(event EventTick
  (params (DeltaSeconds :type Float%20%28single-precision%29)))

(event Input|ActionEvents|InputActionLeft
  (params (Key :type Key%20Structure :default "None"))
  (:Pressed
    (CallFunction|Rotate "NewEnumerator0")
    (Default|HandlePlayerInput (Variables|Default|GetPlatformSpawnerRef) "NewEnumerator0")))

(event Input|ActionEvents|InputActionRight
  (params (Key :type Key%20Structure :default "None"))
  (:Pressed
    (CallFunction|Rotate "NewEnumerator0")
    (Default|HandlePlayerInput (Variables|Default|GetPlatformSpawnerRef) "NewEnumerator1")))

(fn ConstructionScript)

(fn Rotate
  (params (Direction :type Enum_Platform_Direction%20Enum :default "NewEnumerator0"))
  (switch Utilities|FlowControl|Switch|SwitchonEnum_Platform_Direction Direction
    (:NewEnumerator0
      (Transformation|SetRelativeRotation (Variables|Default|GetbasicCharacter) "0,-45.000000, 0" false false))
    (:NewEnumerator1
      (Transformation|SetRelativeRotation (Variables|Default|GetbasicCharacter) "0,-135.000000, 0" false false))))