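; BP_Proto_Platform is a prototype platform for InfiniteSteps that loses durability over time and ends the game when it runs out.
; DecreaseDurability lowers Durability and re-arms itself each second with a timer by function name.
; At zero it clears the timer and calls EndGame on InfiniteStepsGameMode.
; The event graph and construction script are empty, so nothing in this Blueprint starts the countdown.
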(event EventBeginPlay)

(event Collision|EventActorBeginOverlap
  (params (OtherActor :type Actor%20Object%20Reference)))

(event EventTick
  (params (DeltaSeconds :type Float%20%28single-precision%29)))

(fn ConstructionScript)

(fn DecreaseDurability
  (bind _output_get (Variables|Default|SetDurability (- (Variables|Default|GetDurability) 1.0)))
  (if (<= _output_get 0.0)
    (Utilities|Time|ClearandInvalidateTimerbyHandle (Variables|Default|GetT_Durability))
    (bind _asinfinite_steps_game_mode (Utilities|Casting|CastToInfiniteStepsGameMode (Game|GetGameMode)))
    (Default|EndGame _asinfinite_steps_game_mode)
    (else
      (bind _returnvalue (Utilities|Time|SetTimerbyFunctionName 0 "DecreaseDurability" 1.0))
      (Variables|Default|SetT_Durability _returnvalue))))